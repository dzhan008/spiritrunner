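; Base floor tile for an endless runner that randomly populates itself and drives track spawning and cleanup.
; The construction script rolls among blockers, coins, super speed and logs, rerolling on obstacle-history flags.
; When RunCharacter overlaps its Box, the tile joins FloorsPast, then either batch-destroys the oldest tiles or has RunGameMode add one below TileCap.
; GetAttachTransform exposes the AttachPoint's world transform.
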(event OnComponentBeginOverlap(Box)
  (params (OtherActor :type Actor%20Object%20Reference) (OtherComp :type Primitive%20Component%20Object%20Reference) (OtherBodyIndex :type Integer) (bFromSweep :type Boolean) (SweepResult :type Hit%20Result%20Structure%20%28by%20ref%29))
  ;[1 1 1] Sets limit on how many tiles spawned at a time
  (bind _asrun_character (Utilities|Casting|CastToRunCharacter OtherActor))
  ;[1 1 1] Removes tiles after a certain amount of tiles is passed
  (Utilities|Array|Add (Variables|/Game/SpiritRunner/Blueprints/RunCharacter.RunCharacter_C|GetFloorsPast _asrun_character) self)
  (if (< 5 (Utilities|Array|Length (Variables|/Game/SpiritRunner/Blueprints/RunCharacter.RunCharacter_C|GetFloorsPast _asrun_character)))
    (bind _asrun_character_2 (Utilities|Casting|CastToRunCharacter (Game|GetPlayerCharacter 0)))
    (for _index (range 0 4)
      (Actor|DestroyActor (Utilities|Array|Get(acopy) (Variables|/Game/SpiritRunner/Blueprints/RunCharacter.RunCharacter_C|GetFloorsPast _asrun_character_2)))
      (Utilities|Array|RemoveIndex (Variables|/Game/SpiritRunner/Blueprints/RunCharacter.RunCharacter_C|GetFloorsPast _asrun_character_2)))
    (bind _asrun_game_mode (Utilities|Casting|CastToRunGameMode (Game|GetGameMode)))
    ;[1 1 1] Test for This
    (Variables|/Game/SpiritRunner/Blueprints/RunGameMode.RunGameMode_C|SetCurrTiles _asrun_game_mode (- (Variables|/Game/SpiritRunner/Blueprints/RunGameMode.RunGameMode_C|GetCurrTiles _asrun_game_mode) 5))
    (else
      (bind _asrun_game_mode_2 (Utilities|Casting|CastToRunGameMode (Game|GetGameMode)))
      (if (< (Variables|/Game/SpiritRunner/Blueprints/RunGameMode.RunGameMode_C|GetCurrTiles _asrun_game_mode_2) (Variables|/Game/SpiritRunner/Blueprints/RunGameMode.RunGameMode_C|GetTileCap _asrun_game_mode_2))
        (bind _output_get (Variables|/Game/SpiritRunner/Blueprints/RunGameMode.RunGameMode_C|SetCurrTiles _asrun_game_mode_2 (+ (Variables|/Game/SpiritRunner/Blueprints/RunGameMode.RunGameMode_C|GetCurrTiles _asrun_game_mode_2) 1)))
        (Default|AddFloorTile _asrun_game_mode_2)))))

(event OnComponentBeginOverlap(CoinArea)
  (params (OtherActor :type Actor%20Object%20Reference) (OtherComp :type Primitive%20Component%20Object%20Reference) (OtherBodyIndex :type Integer) (bFromSweep :type Boolean) (SweepResult :type Hit%20Result%20Structure%20%28by%20ref%29))
  ;[1 1 1] Sets limit on how many tiles spawned at a time
)

(event EventBeginPlay)

(event Collision|EventActorBeginOverlap
  (params (OtherActor :type Actor%20Object%20Reference)))

(event EventTick
  (params (DeltaSeconds :type Float%20%28single-precision%29))
  ;[1 1 1] Removes tiles after a certain amount of tiles is passed
)

(fn ConstructionScript
  (CallFunction|SetSpawnPoints)
  (switch int (Math|Random|RandomIntegerinRange 0 4) :!label _label
    (:0
      (if (Variables|Default|GetObstacleLastSpawn)
        (goto _label)
        (else
          (CallFunction|SpawnBlocker)
          (Variables|Default|SetObstacleLastSpawn true)
          (Variables|Default|SetLogCounter 0))))
    (:1
      (CallFunction|SpawnCoins)
      (Variables|Default|SetObstacleLastSpawn false)
      (Variables|Default|SetLogCounter (+ (Variables|Default|GetLogCounter) 1)))
    (:2
      (CallFunction|SpawnSuperSpeed)
      (Variables|Default|SetObstacleLastSpawn false)
      (Variables|Default|SetLogCounter (+ (Variables|Default|GetLogCounter) 1)))
    (:3
      (if (and (not (Variables|Default|GetObstacleLastSpawn)) (>= (Variables|Default|GetLogCounter) 3))
        (goto _label)
        (else
          (CallFunction|SpawnLog)
          (Variables|Default|SetObstacleLastSpawn true)
          (Variables|Default|SetLogCounter 0))))
    (:4
      (CallFunction|SpawnBlockers))))

(fn GetAttachTransform
  (return (Transformation|GetWorldTransform (Variables|Default|GetAttachPoint))))

(fn SpawnBlocker
  (bind _spawnpoints (Variables|Default|GetSpawnPoints))
  (AddComponent|AddChildActorComponent false (Utilities|Array|Get(acopy) _spawnpoints (Math|Random|RandomIntegerinRange 0 (Utilities|Array|LastIndex _spawnpoints)))))

(fn SpawnCoins
  (bind _coinarea (Variables|Default|GetCoinArea))
  (for _index (range 0 3)
    (AddComponent|AddChildActorComponent false (Math|Conversions|ToTransform(Vector) (Math|Random|RandomPointinBoundingBox (Variables|/Script/Engine.SceneComponent|GetRelativeLocation _coinarea) (Variables|/Script/Engine.BoxComponent|GetBoxExtent _coinarea))))))

(fn SpawnLog
  ;[1 1 1] Spawns First Set
  (AddComponent|AddChildActorComponent false (Transformation|GetRelativeTransform (Variables|Default|GetSpawnPointLogF)))
  (switch int (Math|Random|RandomIntegerinRange 0 1)
    (:1
      (AddComponent|AddChildActorComponent false (Transformation|GetRelativeTransform (Variables|Default|GetSpawnPointLogB))))))

(fn SpawnSuperSpeed
  (AddComponent|AddChildActorComponent false (Transformation|GetRelativeTransform (Variables|Default|GetSpawnPointSS))))

(fn SetSpawnPoints
  (Variables|Default|SetSpawnPoints (Utilities|Array|MakeArray (Transformation|GetRelativeTransform (Variables|Default|GetSpawnPoint)) (Transformation|GetRelativeTransform (Variables|Default|GetSpawnPointR)) (Transformation|GetRelativeTransform (Variables|Default|GetSpawnPointL)))))

(fn SpawnBlockers
  (switch int (Math|Random|RandomIntegerinRange 0 1)
    (:0
      (AddComponent|AddChildActorComponent false (Transformation|GetRelativeTransform (Variables|Default|GetSpawnPointL)))
      (AddComponent|AddChildActorComponent false (Transformation|GetRelativeTransform (Variables|Default|GetSpawnPointLogB)))
      (AddComponent|AddChildActorComponent false (Transformation|GetRelativeTransform (Variables|Default|GetSpawnPointLogF))))
    (:1
      (AddComponent|AddChildActorComponent false (Transformation|GetRelativeTransform (Variables|Default|GetSpawnPointR)))
      (AddComponent|AddChildActorComponent false (Transformation|GetRelativeTransform (Variables|Default|GetSpawnPointLogB)))
      (AddComponent|AddChildActorComponent false (Transformation|GetRelativeTransform (Variables|Default|GetSpawnPointLogF))))))