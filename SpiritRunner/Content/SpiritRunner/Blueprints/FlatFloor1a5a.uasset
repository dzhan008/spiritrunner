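; Endless-runner floor tile that, when RunCharacter overlaps its Box, asks RunGameMode to add another tile and destroys itself two seconds later.
; Its construction script scatters trees in two box volumes, then randomly adds a three-lane blocker, coins, super speed, logs or nothing as child actors.
; Some obstacle picks reroll based on ObstacleLastSpawn and LogCounter, which are instance variables.
; GetAttachTransform exposes the AttachPoint's world transform.
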(event OnComponentBeginOverlap(Box)
  (params (OtherActor :type Actor%20Object%20Reference) (OtherComp :type Primitive%20Component%20Object%20Reference) (OtherBodyIndex :type Integer) (bFromSweep :type Boolean) (SweepResult :type Hit%20Result%20Structure%20%28by%20ref%29))
  (Utilities|Casting|CastToRunCharacter OtherActor)
  (bind _asrun_game_mode (Utilities|Casting|CastToRunGameMode (Game|GetGameMode)))
  (Default|AddFloorTile _asrun_game_mode)
  (Utilities|FlowControl|Delay 2.0)
  (Actor|DestroyActor))

(event OnComponentBeginOverlap(CoinArea)
  (params (OtherActor :type Actor%20Object%20Reference) (OtherComp :type Primitive%20Component%20Object%20Reference) (OtherBodyIndex :type Integer) (bFromSweep :type Boolean) (SweepResult :type Hit%20Result%20Structure%20%28by%20ref%29)))

(event EventBeginPlay)

(event Collision|EventActorBeginOverlap
  (params (OtherActor :type Actor%20Object%20Reference)))

(event EventTick
  (params (DeltaSeconds :type Float%20%28single-precision%29)))

(fn ConstructionScript
  (CallFunction|SetSpawnPoints)
  (CallFunction|SpawnTrees)
  (switch int (Math|Random|RandomIntegerinRange 0 4) :!label _label
    (:0
      (if (Variables|Default|GetObstacleLastSpawn)
        (goto _label)
        (else
          (CallFunction|SpawnBlocker)
          (Variables|Default|SetObstacleLastSpawn true)
          (Variables|Default|SetLogCounter 0))))
    (:1
      (CallFunction|SpawnCoins)
      (Variables|Default|SetObstacleLastSpawn false)
      (Variables|Default|SetLogCounter (+ (Variables|Default|GetLogCounter) 1)))
    (:2
      (CallFunction|SpawnSuperSpeed)
      (Variables|Default|SetObstacleLastSpawn false)
      (Variables|Default|SetLogCounter (+ (Variables|Default|GetLogCounter) 1)))
    (:3
      (if (and (not (Variables|Default|GetObstacleLastSpawn)) (>= (Variables|Default|GetLogCounter) 3))
        (goto _label)
        (else
          (CallFunction|SpawnLog)
          (Variables|Default|SetObstacleLastSpawn true)
          (Variables|Default|SetLogCounter 0))))))

(fn SpawnTrees
  (bind _treespawn1 (Variables|Default|GetTreeSpawn1))
  (bind _treespawn2 (Variables|Default|GetTreeSpawn2))
  (for _index (range 0 (Variables|Default|GetMaxTrees))
    (AddComponent|AddChildActorComponent false (Math|Conversions|ToTransform(Vector) (Math|Random|RandomPointinBoundingBox (Variables|/Script/Engine.SceneComponent|GetRelativeLocation _treespawn1) (Variables|/Script/Engine.BoxComponent|GetBoxExtent _treespawn1))))
    (AddComponent|AddChildActorComponent false (Math|Conversions|ToTransform(Vector) (Math|Random|RandomPointinBoundingBox (Variables|/Script/Engine.SceneComponent|GetRelativeLocation _treespawn2) (Variables|/Script/Engine.BoxComponent|GetBoxExtent _treespawn2))))))

(fn GetAttachTransform
  (return (Transformation|GetWorldTransform (Variables|Default|GetAttachPoint))))

(fn SpawnBlocker
  (bind _spawnpoints (Variables|Default|GetSpawnPoints))
  (AddComponent|AddChildActorComponent false (Utilities|Array|Get(acopy) _spawnpoints (Math|Random|RandomIntegerinRange 0 (Utilities|Array|LastIndex _spawnpoints)))))

(fn SpawnCoins
  (bind _coinarea (Variables|Default|GetCoinArea))
  (for _index (range 0 3)
    (AddComponent|AddChildActorComponent false (Math|Conversions|ToTransform(Vector) (Math|Random|RandomPointinBoundingBox (Variables|/Script/Engine.SceneComponent|GetRelativeLocation _coinarea) (Variables|/Script/Engine.BoxComponent|GetBoxExtent _coinarea))))))

(fn SpawnLog
  ;[1 1 1] Spawns First Set
  (AddComponent|AddChildActorComponent false (Transformation|GetRelativeTransform (Variables|Default|GetSpawnPointLogF)))
  (switch int (Math|Random|RandomIntegerinRange 0 1)
    (:1
      (AddComponent|AddChildActorComponent false (Transformation|GetRelativeTransform (Variables|Default|GetSpawnPointLogB))))))

(fn SpawnSuperSpeed
  (AddComponent|AddChildActorComponent false (Transformation|GetRelativeTransform (Variables|Default|GetSpawnPointSS))))

(fn SetSpawnPoints
  (Variables|Default|SetSpawnPoints (Utilities|Array|MakeArray (Transformation|GetRelativeTransform (Variables|Default|GetSpawnPoint)) (Transformation|GetRelativeTransform (Variables|Default|GetSpawnPointR)) (Transformation|GetRelativeTransform (Variables|Default|GetSpawnPointL)))))