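; FlatFloor1 is a flat floor segment for SpiritRunner that scatters trees when constructed.
; The construction script calls SpawnTrees, which loops up to MaxTrees, adding child actors at random points inside the TreeSpawn1 and TreeSpawn2 boxes.
; GetAttachTransform returns the AttachPoint's world transform, exposing an attachment point on the segment.
; The event graph has no active logic.
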(event EventBeginPlay)

(event Collision|EventActorBeginOverlap
  (params (OtherActor :type Actor%20Object%20Reference)))

(event EventTick
  (params (DeltaSeconds :type Float%20%28single-precision%29)))

(fn ConstructionScript
  (CallFunction|SpawnTrees))

(fn SpawnTrees
  (bind _treespawn1 (Variables|Default|GetTreeSpawn1))
  (bind _treespawn2 (Variables|Default|GetTreeSpawn2))
  (for _index (range 0 (Variables|Default|GetMax%20Trees))
    (AddComponent|AddChildActorComponent false (Math|Conversions|ToTransform(Vector) (Math|Random|RandomPointinBoundingBox (Variables|/Script/Engine.SceneComponent|GetRelativeLocation _treespawn1) (Variables|/Script/Engine.BoxComponent|GetBoxExtent _treespawn1))))
    (AddComponent|AddChildActorComponent false (Math|Conversions|ToTransform(Vector) (Math|Random|RandomPointinBoundingBox (Variables|/Script/Engine.SceneComponent|GetRelativeLocation _treespawn2) (Variables|/Script/Engine.BoxComponent|GetBoxExtent _treespawn2))))))

(fn GetAttachTransform
  (return (Transformation|GetWorldTransform (Variables|Default|GetAttachPoint))))