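; Flat floor tile Blueprint for SpiritRunner with a trigger box that acts as a speed boost for the runner.
; When a RunCharacter overlaps Box1, its max walk speed rises by a fixed amount, with no reset in this Blueprint.
; It then spawns placeholder explosion emitters on either side of player 0 along world Y and prints debug messages.
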(event OnComponentBeginOverlap(Box1)
  (params (OtherActor :type Actor%20Object%20Reference) (OtherComp :type Primitive%20Component%20Object%20Reference) (OtherBodyIndex :type Integer) (bFromSweep :type Boolean) (SweepResult :type Hit%20Result%20Structure%20%28by%20ref%29))
  (bind _asrun_character (Utilities|Casting|CastToRunCharacter OtherActor))
  (Variables|/Script/Engine.CharacterMovementComponent|SetMaxWalkSpeed (Variables|/Script/Engine.Character|GetCharacterMovement _asrun_character) (+ (Variables|/Script/Engine.CharacterMovementComponent|GetMaxWalkSpeed (Variables|/Script/Engine.Character|GetCharacterMovement _asrun_character)) 2e+02))
  (bind _asrun_character_2 (Utilities|Casting|CastToRunCharacter (Game|GetPlayerCharacter 0)))
  (Effects|SpawnEmitteratLocation "/Game/StarterContent/Particles/P_Explosion.P_Explosion" (Math|Vector|MakeVector (.X (Math|Vector|BreakVector (Transformation|GetActorLocation _asrun_character_2))) (- (.Y (Math|Vector|BreakVector (Transformation|GetActorLocation _asrun_character_2))) 1e+02) (.Z (Math|Vector|BreakVector (Transformation|GetActorLocation _asrun_character_2)))))
  (Effects|SpawnEmitteratLocation "/Game/StarterContent/Particles/P_Explosion.P_Explosion" (Math|Vector|MakeVector (.X (Math|Vector|BreakVector (Transformation|GetActorLocation _asrun_character_2))) (+ (.Y (Math|Vector|BreakVector (Transformation|GetActorLocation _asrun_character_2))) 1e+02) (.Z (Math|Vector|BreakVector (Transformation|GetActorLocation _asrun_character_2)))))
  (Development|PrintString "*Insert Flashy Particle Effect Here*")
  (Development|PrintString "Speed Increased!"))

(event EventBeginPlay)

(event Collision|EventActorBeginOverlap
  (params (OtherActor :type Actor%20Object%20Reference)))

(event EventTick
  (params (DeltaSeconds :type Float%20%28single-precision%29)))

(fn ConstructionScript)