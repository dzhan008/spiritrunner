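; Flat floor tile Blueprint for SpiritRunner that scatters bamboo across itself procedurally.
; Its construction script calls SpawnBamboo, then runs the parent construction script.
; SpawnBamboo loops to add child actor components at random points inside the BambooArea box, giving each spawned actor a random yaw.
; Placement is unseeded, so the layout changes whenever construction reruns; the event graph is empty.
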(event EventBeginPlay)

(event Collision|EventActorBeginOverlap
  (params (OtherActor :type Actor%20Object%20Reference)))

(event EventTick
  (params (DeltaSeconds :type Float%20%28single-precision%29)))

(fn ConstructionScript
  (CallFunction|SpawnBamboo)
  (|CallParentFunction))

(fn SpawnBamboo
  (bind _bamboo_area (Variables|Default|GetBamboo%20Area))
  (for _index (range 0 60)
    (bind _returnvalue (AddComponent|AddChildActorComponent false (Math|Conversions|ToTransform(Vector) (Math|Random|RandomPointinBoundingBox (Variables|/Script/Engine.SceneComponent|GetRelativeLocation _bamboo_area) (Variables|/Script/Engine.BoxComponent|GetBoxExtent _bamboo_area)))))
    (Transformation|SetActorRotation (Variables|/Script/Engine.ChildActorComponent|GetChildActor _returnvalue) (Class|KismetMathLibrary|MakeRot 0.0 (+ 0.0 (Math|Random|RandomFloatinRange 0.0 3.6e+02)) 0.0))))