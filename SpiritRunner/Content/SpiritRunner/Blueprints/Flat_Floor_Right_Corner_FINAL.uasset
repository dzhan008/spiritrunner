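; Flat right-corner floor tile for an endless runner, where the player is allowed to turn.
; An exit trigger (Box1) has RunGameMode add the next tile, then destroys this one after a short delay.
; TurnZone sets CanTurn on the RunCharacter when it enters.
; Five wall components each call Death on the character when the hit normal nearly aligns with its forward vector, using a dot-product test.
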(event OnComponentHit(Wall)
  (params (OtherActor :type Actor%20Object%20Reference) (OtherComp :type Primitive%20Component%20Object%20Reference) (NormalImpulse :type Vector :default "0, 0, 0") (Hit :type Hit%20Result%20Structure%20%28by%20ref%29))
  ;[1 1 1] Hit a Wall
  (bind _asrun_character (Utilities|Casting|CastToRunCharacter OtherActor))
  (if (Math|Float|NearlyEqual(Float) (Math|Vector|DotProduct (.normal Hit) (Transformation|GetActorForwardVector _asrun_character)) 1.0 0.1)
    (Default|Death _asrun_character)))

(event OnComponentHit(Wall2_0)
  (params (OtherActor :type Actor%20Object%20Reference) (OtherComp :type Primitive%20Component%20Object%20Reference) (NormalImpulse :type Vector :default "0, 0, 0") (Hit :type Hit%20Result%20Structure%20%28by%20ref%29))
  ;[1 1 1] Hit a Wall
  (bind _asrun_character (Utilities|Casting|CastToRunCharacter OtherActor))
  (if (Math|Float|NearlyEqual(Float) (Math|Vector|DotProduct (.normal Hit) (Transformation|GetActorForwardVector _asrun_character)) 1.0 0.1)
    (Default|Death _asrun_character)))

(event OnComponentHit(Wall3)
  (params (OtherActor :type Actor%20Object%20Reference) (OtherComp :type Primitive%20Component%20Object%20Reference) (NormalImpulse :type Vector :default "0, 0, 0") (Hit :type Hit%20Result%20Structure%20%28by%20ref%29))
  (bind _asrun_character (Utilities|Casting|CastToRunCharacter OtherActor))
  (if (Math|Float|NearlyEqual(Float) (Math|Vector|DotProduct (.normal Hit) (Transformation|GetActorForwardVector _asrun_character)) 1.0 0.1)
    (Default|Death _asrun_character)))

(event OnComponentBeginOverlap(Box1)
  (params (OtherActor :type Actor%20Object%20Reference) (OtherComp :type Primitive%20Component%20Object%20Reference) (OtherBodyIndex :type Integer) (bFromSweep :type Boolean) (SweepResult :type Hit%20Result%20Structure%20%28by%20ref%29))
  (Utilities|Casting|CastToRunCharacter OtherActor)
  (bind _asrun_game_mode (Utilities|Casting|CastToRunGameMode (Game|GetGameMode)))
  (Default|AddFloorTile _asrun_game_mode)
  (Utilities|FlowControl|Delay 2.0)
  (Actor|DestroyActor))

(event OnComponentHit(Wall4)
  (params (OtherActor :type Actor%20Object%20Reference) (OtherComp :type Primitive%20Component%20Object%20Reference) (NormalImpulse :type Vector :default "0, 0, 0") (Hit :type Hit%20Result%20Structure%20%28by%20ref%29))
  (bind _asrun_character (Utilities|Casting|CastToRunCharacter OtherActor))
  (if (Math|Float|NearlyEqual(Float) (Math|Vector|DotProduct (.normal Hit) (Transformation|GetActorForwardVector _asrun_character)) 1.0 0.1)
    (Default|Death _asrun_character)))

(event OnComponentBeginOverlap(TurnZone)
  (params (OtherActor :type Actor%20Object%20Reference) (OtherComp :type Primitive%20Component%20Object%20Reference) (OtherBodyIndex :type Integer) (bFromSweep :type Boolean) (SweepResult :type Hit%20Result%20Structure%20%28by%20ref%29))
  (bind _asrun_character (Utilities|Casting|CastToRunCharacter OtherActor))
  (Variables|/Game/SpiritRunner/Blueprints/RunCharacter.RunCharacter_C|SetCanTurn _asrun_character true))

(event OnComponentHit(Wall1)
  (params (OtherActor :type Actor%20Object%20Reference) (OtherComp :type Primitive%20Component%20Object%20Reference) (NormalImpulse :type Vector :default "0, 0, 0") (Hit :type Hit%20Result%20Structure%20%28by%20ref%29))
  (bind _asrun_character (Utilities|Casting|CastToRunCharacter OtherActor))
  (if (Math|Float|NearlyEqual(Float) (Math|Vector|DotProduct (.normal Hit) (Transformation|GetActorForwardVector _asrun_character)) 1.0 0.1)
    (Default|Death _asrun_character)))

(event EventBeginPlay)

(event Collision|EventActorBeginOverlap
  (params (OtherActor :type Actor%20Object%20Reference)))

(event EventTick
  (params (DeltaSeconds :type Float%20%28single-precision%29)))

(fn ConstructionScript)