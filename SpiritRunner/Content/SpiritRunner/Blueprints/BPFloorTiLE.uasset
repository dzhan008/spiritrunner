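; Floor tile for an endless runner that asks RunGameMode to add another tile when RunCharacter reaches EndTrigger, then destroys itself two seconds later.
; The construction script randomly spawns a blocker, coins, super speed pickup or log obstacle as child actors, re-rolling obstacle picks while ObstacleSpawn is set.
; Two wall components kill the runner when the hit normal nearly aligns with its forward vector.
; GetAttachTransform exposes the AttachPoint transform.
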(event OnComponentBeginOverlap(EndTrigger)
  (params (OtherActor :type Actor%20Object%20Reference) (OtherComp :type Primitive%20Component%20Object%20Reference) (OtherBodyIndex :type Integer) (bFromSweep :type Boolean) (SweepResult :type Hit%20Result%20Structure%20%28by%20ref%29))
  (Utilities|Casting|CastToRunCharacter OtherActor)
  (bind _asrun_game_mode (Utilities|Casting|CastToRunGameMode (Game|GetGameMode)))
  (Default|AddFloorTile _asrun_game_mode)
  (Utilities|FlowControl|Delay 2.0)
  (Actor|DestroyActor))

(event OnComponentHit(Wall)
  (params (OtherActor :type Actor%20Object%20Reference) (OtherComp :type Primitive%20Component%20Object%20Reference) (NormalImpulse :type Vector :default "0, 0, 0") (Hit :type Hit%20Result%20Structure%20%28by%20ref%29))
  ;[1 1 1] Hit a Wall
  (bind _asrun_character (Utilities|Casting|CastToRunCharacter OtherActor))
  (if (Math|Float|NearlyEqual(Float) (Math|Vector|DotProduct (.normal Hit) (Transformation|GetActorForwardVector _asrun_character)) 1.0 0.1)
    (Default|Death _asrun_character)))

(event OnComponentHit(Wall2)
  (params (OtherActor :type Actor%20Object%20Reference) (OtherComp :type Primitive%20Component%20Object%20Reference) (NormalImpulse :type Vector :default "0, 0, 0") (Hit :type Hit%20Result%20Structure%20%28by%20ref%29))
  ;[1 1 1] Hit a Wall
  (bind _asrun_character (Utilities|Casting|CastToRunCharacter OtherActor))
  (if (Math|Float|NearlyEqual(Float) (Math|Vector|DotProduct (.normal Hit) (Transformation|GetActorForwardVector _asrun_character)) 1.0 0.1)
    (Default|Death _asrun_character)))

(event EventBeginPlay)

(event Collision|EventActorBeginOverlap
  (params (OtherActor :type Actor%20Object%20Reference)))

(event EventTick
  (params (DeltaSeconds :type Float%20%28single-precision%29)))

(fn ConstructionScript
  (CallFunction|SetSpawnPoints)
  (switch int (Math|Random|RandomIntegerinRange 0 3) :!label _label
    (:0
      (if (Variables|Default|GetObstacleSpawn)
        (goto _label)
        (else
          (CallFunction|SpawnBlocker)
          (Variables|Default|SetObstacleSpawn true))))
    (:1
      (CallFunction|SpawnCoins)
      (Variables|Default|SetObstacleSpawn false))
    (:2
      (CallFunction|SpawnSuperSpeed)
      (Variables|Default|SetObstacleSpawn false))
    (:3
      (if (Variables|Default|GetObstacleSpawn)
        (goto _label)
        (else
          (CallFunction|SpawnLogObstacle)
          (Variables|Default|SetObstacleSpawn true))))))

(fn GetAttachTransform
  (return (Transformation|GetWorldTransform (Variables|Default|GetAttachPoint))))

(fn SetSpawnPoints
  (Variables|Default|SetSpawnPoints (Utilities|Array|MakeArray (Transformation|GetRelativeTransform (Variables|Default|GetSpawnPoint)) (Transformation|GetRelativeTransform (Variables|Default|GetSpawnPointR)) (Transformation|GetRelativeTransform (Variables|Default|GetSpawnPointL)))))

(fn SpawnBlocker
  (bind _spawnpoints (Variables|Default|GetSpawnPoints))
  (AddComponent|AddChildActorComponent false (Utilities|Array|Get(acopy) _spawnpoints (Math|Random|RandomIntegerinRange 0 (Utilities|Array|LastIndex _spawnpoints)))))

(fn SpawnCoins
  (bind _coin_area (Variables|Default|GetCoin%20Area))
  (for _index (range 0 3)
    (AddComponent|AddChildActorComponent false (Math|Conversions|ToTransform(Vector) (Math|Random|RandomPointinBoundingBox (Variables|/Script/Engine.SceneComponent|GetRelativeLocation _coin_area) (Variables|/Script/Engine.BoxComponent|GetBoxExtent _coin_area))))))

(fn SpawnSuperSpeed
  (AddComponent|AddChildActorComponent false (Transformation|GetRelativeTransform (Variables|Default|GetSpawnPointSS))))

(fn SpawnLogObstacle
  (AddComponent|AddChildActorComponent false (Transformation|GetRelativeTransform (Variables|Default|GetSpawnPointSS))))