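; Game mode for an endless runner that shows the main menu with music, pre-spawns the track and holds the player still.
; Floor tiles chain by attach transforms from a starting shrine.
; AddFloorTile places random straights, or a torii gate whenever the player's distance passes a goal that rises per gate.
; Past a straight limit it spawns a random curve and redraws the limit, withholding the last pick to avoid repeats.
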(event EventBeginPlay
  (bind _returnvalue (Game|GetPlayerCharacter 0))
  (Input|SetInputModeUIOnly 0 0 false)
  (bind _returnvalue_2 (UserInterface|CreateWidget "/Game/SpiritRunner/UMG/MainMenu.MainMenu_C"))
  (UserInterface|Viewport|AddtoViewport _returnvalue_2 0)
  (bind _returnvalue_3 (AddComponent|AddAudioComponent false))
  (Audio|Components|Audio|Play (Variables|Default|GetMenuSong) 0.0)
  (Variables|/Script/Engine.PlayerController|SetbShowMouseCursor (Game|GetPlayerController 0) true)
  (CallFunction|AddFirstFloorTile)
  (for _index (range 0 4)
    (bind _asrun_character (Utilities|Casting|CastToRunCharacter _returnvalue))
    (Development|PrintString "second for loop add tail")
    (CallFunction|AddFloorTile)
    (for _index_2 (range 0 (Variables|/Game/SpiritRunner/Blueprints/RunCharacter.RunCharacter_C|GetToriGateSpawnRate _asrun_character))
      (CallFunction|AddFloorTile))
    (bind _asrun_character_2 (Utilities|Casting|CastToRunCharacter _returnvalue))
    (Components|Movement|StopMovementImmediately (Variables|/Script/Engine.Character|GetCharacterMovement _asrun_character_2))
    (Variables|/Script/Engine.CharacterMovementComponent|SetMaxWalkSpeed (Variables|/Script/Engine.Character|GetCharacterMovement _asrun_character_2) 0.0))
  (bind _asrun_character_3 (Utilities|Casting|CastToRunCharacter _returnvalue))
  (Components|Movement|StopMovementImmediately (Variables|/Script/Engine.Character|GetCharacterMovement _asrun_character_3))
  (Variables|/Script/Engine.CharacterMovementComponent|SetMaxWalkSpeed (Variables|/Script/Engine.Character|GetCharacterMovement _asrun_character_3) 0.0))

(event EventTick
  (params (DeltaSeconds :type Float%20%28single-precision%29))
  (if (Variables|Default|GetStartGame)
    (Audio|Components|Audio|Stop (stale EventBeginPlay _returnvalue_3))))

(fn ConstructionScript)

(fn AddFloorTile
  (bind _returnvalue (Game|GetPlayerCharacter 0))
  (bind _floortiles (Variables|Default|GetFloorTiles))
  (bind _output_get (Variables|Default|SetTILE_COUNT (+ (Variables|Default|GetTILE_COUNT) 1)))
  (Development|PrintString (Utilities|String|ToString(Integer) _output_get))
  (if (> (Variables|Default|GetCurrentStraights) (Variables|Default|GetMaxStraights))
    (CallFunction|AddFloorCorner)
    (else
      (bind _asrun_character (Utilities|Casting|CastToRunCharacter _returnvalue))
      ;[1 1 1] Spawns Torigate and makes a new distance
      (if (< (Variables|/Game/SpiritRunner/Blueprints/RunCharacter.RunCharacter_C|GetGoalDistance _asrun_character) (Variables|/Game/SpiritRunner/Blueprints/RunCharacter.RunCharacter_C|GetTotalDistance _asrun_character))
        (bind _asrun_character_2 (Utilities|Casting|CastToRunCharacter _returnvalue))
        (Variables|/Game/SpiritRunner/Blueprints/RunCharacter.RunCharacter_C|SetGoalDistance _asrun_character_2 (+ (Variables|/Game/SpiritRunner/Blueprints/RunCharacter.RunCharacter_C|GetGoalDistance _asrun_character_2) 1000))
        (bind _returnvalue_2 (Game|SpawnActorfromClass "/Game/SpiritRunner/Blueprints/Flat_Floor_Tori.Flat_Floor_Tori_C" (Variables|Default|GetNextSpawnPoint) false 0 0))
        (bind _attachtransform (Default|GetAttachTransform _returnvalue_2))
        (Variables|Default|SetNextSpawnPoint _attachtransform)
        (else
          (bind _returnvalue_3 (Game|SpawnActorfromClass (Utilities|Array|Get(acopy) _floortiles (Math|Random|RandomIntegerinRange 0 (Utilities|Array|LastIndex _floortiles))) (Variables|Default|GetNextSpawnPoint) false 0 0))
          (bind _asflat_floor_base (Utilities|Casting|CastToFlat_Floor_BASE _returnvalue_3))
          (bind _attachtransform_2 (Default|GetAttachTransform _asflat_floor_base))
          (Variables|Default|SetNextSpawnPoint _attachtransform_2)))
      ;[1 1 1] Add to straight counter
      (Variables|Default|SetCurrentStraights (+ (Variables|Default|GetCurrentStraights) 1)))))

(fn AddFloorCorner
  (bind _floorcurves (Variables|Default|GetFloorCurves))
  (bind _returnvalue (Game|SpawnActorfromClass (Utilities|Array|Get(acopy) _floorcurves (Math|Random|RandomIntegerinRange 0 (Utilities|Array|LastIndex _floorcurves))) (Variables|Default|GetNextSpawnPoint) false 0 0))
  (bind _asflat_floor_base (Utilities|Casting|CastToFlat_Floor_BASE _returnvalue))
  (bind _attachtransform (Default|GetAttachTransform _asflat_floor_base))
  (Variables|Default|SetNextSpawnPoint _attachtransform)
  (Variables|Default|SetCurrentStraights 0)
  (CallFunction|SetNewMaxStraights))

(fn AddFirstFloorTile
  (bind _returnvalue (Game|SpawnActorfromClass "/Game/SpiritRunner/Blueprints/Shrine_Spawn.Shrine_Spawn_C" (Variables|Default|GetNextSpawnPoint) false 0 0))
  (bind _attachtransform (Default|GetAttachTransform _returnvalue))
  (bind _output_get (Variables|Default|SetNextSpawnPoint _attachtransform))
  (bind _returnvalue_2 (Game|SpawnActorfromClass "/Game/SpiritRunner/Blueprints/Flat_Floor_Flat.Flat_Floor_Flat_C" _output_get false 0 0))
  (bind _attachtransform_2 (Default|GetAttachTransform _returnvalue_2))
  (Variables|Default|SetNextSpawnPoint _attachtransform_2))

(fn SetNewMaxStraights
  (bind _straightnum (Variables|Default|GetStraightNum))
  (Variables|Default|SetMaxStraights (Utilities|Array|Get(acopy) _straightnum (Math|Random|RandomIntegerinRange 0 (Utilities|Array|LastIndex _straightnum))))
  (Utilities|Array|Add _straightnum (Variables|Default|GetPlaceholder))
  (Variables|Default|SetPlaceholder (Variables|Default|GetMaxStraights))
  (Utilities|Array|RemoveItem _straightnum (Variables|Default|GetMaxStraights)))